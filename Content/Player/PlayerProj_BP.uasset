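; PlayerProj_BP is the player's projectile, which damages AI characters it overlaps.
; The construction script tints the mesh material using the ProjectileColor of the owning PlayerChar_BP.
; The first overlap with an AIChar_BP applies the owner's Damage through a DoOnce gate, then destroys the projectile.
; Other actors are ignored, and the projectile destroys itself after a short lifetime delay from BeginPlay.
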(event `self.ReceiveBeginPlay`
  (`KismetSystemLibrary.Delay` 3.0)
  (`self.K2_DestroyActor`))

(event `self.ProjectileOverlap.OnComponentBeginOverlap`
  (params (OverlappedComponent :type "PrimitiveComponent Object Reference") (OtherActor :type "Actor Object Reference") (OtherComp :type "PrimitiveComponent Object Reference") (OtherBodyIndex :type Integer) (bFromSweep :type Boolean) (SweepResult :type "HitResult Structure (by ref)"))
  (bind _asaichar_bp (cast `/Game/AI/AIChar_BP` OtherActor))
  (`/Engine/EditorBlueprintResources/StandardMacros.DoOnce` false
    (:`Completed`
      (bind _asplayer_char_bp (cast `/Game/Player/PlayerChar_BP` (`self.GetOwner`)))
      (`GameplayStatics.ApplyDamage` _asaichar_bp (`/Game/Player/Char_BP_M.Damage` _asplayer_char_bp) null _asplayer_char_bp)
      (`self.K2_DestroyActor`))))

(fn `UserConstructionScript`
  (bind _asplayer_char_bp (cast `/Game/Player/PlayerChar_BP` (`self.GetOwner`)))
  (`MeshComponent.SetColorParameterValueOnMaterials` (`self.ProjectileMesh`) "Color" (`KismetMathLibrary.Conv_ColorToLinearColor` (`/Game/Player/Char_BP_M.ProjectileColor` _asplayer_char_bp))))